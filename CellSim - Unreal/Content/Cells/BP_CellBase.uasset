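; Base cell actor that grows and reproduces by budding child cells of the same class, driven by CellComponent state.
; A full-grown cell attaches a zero-scale child in a random direction; Tick scales it up and pushes it outward.
; At detach time the child separates, prompting the parent to bud again, and keeps growing until mature.
; InitCell samples growth time from a DataTable by binary search on a random value, deriving detach time from it.
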(event Custom|BeginGrowth
  (if (Variables|/Game/Cells/BP_CellComponent.BP_CellComponent_C|GetbFullGrown? (Variables|Default|GetCellComponent))
    (CallFunction|CreateSon)
    (else
      (Variables|Default|SetbGrowing true))))

(event EventTick
  (params (DeltaSeconds :type Float%20%28single-precision%29))
  (if (Variables|Default|GetbGrowing)
    (CallFunction|Growth)))

(fn ConstructionScript)

(fn CreateSon
  ;[1 1 1] Create Son If Has Not Son Attach
  (bind _returnvalue (Game|SpawnActorfromClass "BP_CellBase_C" (Math|Transform|MakeTransform "20000.000000,20000.000000,20000.000000" "0, 0, 0" "0.000000,0.000000,0.000000") "Undefined" "OverrideRootScale" 0 0))
  ;[1 1 1] Set Reference Of The Son
  (bind _output_get (LocalVariables|SetL_Son _returnvalue))
  (Variables|/Game/Cells/BP_CellComponent.BP_CellComponent_C|SetSon (Variables|Default|GetCellComponent) _output_get)
  ;[1 1 1] Set Relative Position And Attach
  (bind _output_get_2 (Variables|/Game/Cells/BP_CellComponent.BP_CellComponent_C|SetRelativeDirection (Variables|BP_CellBase_C|GetCellComponent (LocalVariables|GetL_Son)) (Math|Random|RandomUnitVector)))
  (bind _output_get_3 (LocalVariables|SetL_Direction (* _output_get_2 24.0)))
  (Variables|/Game/Cells/BP_CellComponent.BP_CellComponent_C|SetRelativePosition (Variables|BP_CellBase_C|GetCellComponent (LocalVariables|GetL_Son)) _output_get_3)
  (Transformation|SetActorLocation (LocalVariables|GetL_Son) (+ (Transformation|GetActorLocation self) (LocalVariables|GetL_Direction)) false true)
  (Transformation|AttachActorToActor (LocalVariables|GetL_Son) self "None" "KeepWorld" "KeepWorld" "KeepWorld" true)
  ;[1 1 1] Set Reference Of Father Cell For The Son And Begin Growth
  (Variables|/Game/Cells/BP_CellComponent.BP_CellComponent_C|SetParent (Variables|BP_CellBase_C|GetCellComponent (LocalVariables|GetL_Son)) self)
  (CallFunction|InitCell (Variables|Initialization|GetDeltaTime))
  (CallFunction|BeginGrowth (LocalVariables|GetL_Son)))

(fn Growth
  (bind _cellcomponent (Variables|Default|GetCellComponent))
  ;[1 1 1] Inicializar Variables
  (LocalVariables|SetActualTime (Default|GetCurrentTime (Variables|Default|GetCellComponent)))
  (LocalVariables|SetMaxTime (Default|GetGrowthTime (Variables|Default|GetCellComponent)))
  ;[1 1 1] Aumentar Tiempo Actual y Aumentar Tamaño
  (Default|ModifyStatGrowing (Variables|Default|GetCellComponent) (Variables|Initialization|GetDeltaTime))
  (Transformation|SetActorScale3D self (Math|Conversions|ToVector(Float) (/ (LocalVariables|GetActualTime) (LocalVariables|GetMaxTime))))
  ;[1 1 1] Verificar si está aún con el padre
  (Utilities|IsValid (Variables|/Game/Cells/BP_CellComponent.BP_CellComponent_C|GetParent (Variables|Default|GetCellComponent))
    (:Is%20Valid
      ;[1 1 1] Situar objeto en nueva posición relativa
      (bind _output_get (Variables|/Game/Cells/BP_CellComponent.BP_CellComponent_C|SetRelativePosition (Variables|Default|GetCellComponent) (+ (* (Variables|/Game/Cells/BP_CellComponent.BP_CellComponent_C|GetRelativeDirection _cellcomponent) (* (/ (Variables|Initialization|GetDeltaTime) (Variables|Initialization|GetTDetach%20Parent%20Time)) 55.0)) (Variables|/Game/Cells/BP_CellComponent.BP_CellComponent_C|GetRelativePosition _cellcomponent))))
      (Transformation|SetActorRelativeLocation self _output_get)
      ;[1 1 1] Verificar separación del padre
      (if (>= (LocalVariables|GetActualTime) (Default|GetDetachParentTime (Variables|Default|GetCellComponent)))
        (CallFunction|DetachfromParent)))
    (:Is%20Not%20Valid
      ;[1 1 1] Verificar si está completamente crecida
      (if (>= (LocalVariables|GetActualTime) (Default|GetGrowthTime (Variables|Default|GetCellComponent)))
        ;[1 1 1] Parar crecimiento y empezar la reproducción
        (Variables|Default|SetbGrowing false)
        (Variables|/Game/Cells/BP_CellComponent.BP_CellComponent_C|SetbFullGrown? (Variables|Default|GetCellComponent) true)
        (CallFunction|BeginGrowth)))))

(fn DetachfromParent
  (Utilities|IsValid (Variables|/Game/Cells/BP_CellComponent.BP_CellComponent_C|GetParent (Variables|Default|GetCellComponent))
    (:Is%20Valid
      (Transformation|DetachFromActor self "KeepWorld" "KeepWorld" "KeepWorld")
      (CallFunction|BeginGrowth (Variables|/Game/Cells/BP_CellComponent.BP_CellComponent_C|GetParent (Variables|Default|GetCellComponent)))
      (Variables|/Game/Cells/BP_CellComponent.BP_CellComponent_C|SetParent (Variables|Default|GetCellComponent) 0)
      (CallFunction|BeginGrowth))))

(fn GenerateGrowthTime
  (params (CellDensityTable :type Data%20Table%20Object%20Reference))
  (LocalVariables|SetRandomVal (Math|Random|RandomFloatinRange 0.0 1.0))
  (bind _returnvalue (Class|DataTableFunctionLibrary|GetDataTableColumnasString CellDensityTable "Min"))
  (LocalVariables|SetMin _returnvalue)
  (bind _returnvalue_2 (Class|DataTableFunctionLibrary|GetDataTableColumnasString CellDensityTable "Var"))
  (bind _output_get (LocalVariables|SetVar _returnvalue_2))
  (LocalVariables|SetEndIndex (Utilities|Array|LastIndex _output_get))
  (if (<= (LocalVariables|GetStartIndex) (LocalVariables|GetEndIndex)) :!label _label
    (LocalVariables|SetMid (/ (+ (LocalVariables|GetStartIndex) (LocalVariables|GetEndIndex)) 2))
    (if (< (Math|Conversions|ToFloat(Integer) (Utilities|Array|Get(acopy) (LocalVariables|GetVar) (LocalVariables|GetMid))) (LocalVariables|GetRandomVal))
      (LocalVariables|SetStartIndex (+ (LocalVariables|GetMid) 1))
      (goto _label)
      (else
        (LocalVariables|SetEndIndex (- (LocalVariables|GetMid) 1))
        (goto _label)))
    (else
      (return (LocalVariables|GetStartIndex)))))

(fn InitCell
  (params (DeltaTime :type Float%20%28double-precision%29))
  (bind _datagrowthtimes (Variables|Default|GetDataGrowthTimes))
  (Variables|Initialization|SetDeltaTime DeltaTime)
  (bind _returnvalue (CallFunction|GenerateGrowthTime _datagrowthtimes))
  (bind _returnvalue_2 (Class|DataTableFunctionLibrary|GetDataTableColumnasString _datagrowthtimes "Min"))
  (bind _output_get (Variables|Initialization|SetTGrowth%20Time (Math|Conversions|ToFloat(Integer) (Utilities|Array|Get(acopy) _returnvalue_2 _returnvalue))))
  (Variables|Initialization|SetTDetach%20Parent%20Time (* _output_get 0.7))
  (Default|StatInitialization (Variables|Default|GetCellComponent) (Variables|Initialization|GetTMax%20Mass) (Variables|Initialization|GetTGrowth%20Time) (Variables|Initialization|GetTDetach%20Parent%20Time))
  (return))