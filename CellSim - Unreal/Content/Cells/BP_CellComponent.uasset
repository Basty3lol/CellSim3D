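; BP_CellComponent stores a cell's growth stats: max mass, total growth time, detach-from-parent time and current time.
; StatInitialization sets the first three through setters that only prevent negative values, as each clamp's upper bound is the input itself.
; ModifyStatGrowing adds a time delta to current time, clamped between zero and total growth time.
; The component has no active event logic, so growth advances only when that function is called.
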(event EventBeginPlay)

(event EventTick
  (params (DeltaSeconds :type Float%20%28single-precision%29)))

(fn SetGrowthTime
  (params (GrowthTime :type Float%20%28double-precision%29))
  (Variables|Initialization|SetTotalGrowthTime (Math|Float|Clamp(Float) GrowthTime 0.0 GrowthTime)))

(fn GetGrowthTime
  (return (Variables|Initialization|GetTotalGrowthTime)))

(fn SetMaxMass
  (params (MaxMass :type Float%20%28double-precision%29))
  (Variables|Initialization|SetMaxMass (Math|Float|Clamp(Float) MaxMass 0.0 MaxMass)))

(fn GetMaxMass
  (return (Variables|Initialization|GetMaxMass)))

(fn ModifyStatGrowing
  (params (DTime :type Float%20%28double-precision%29))
  (bind _output_get (LocalVariables|SetNewTime (+ (Variables|Default|GetCurrentTime) DTime)))
  (Growing|SetCurrentTime (Math|Float|Clamp(Float) _output_get 0.0 (Variables|Initialization|GetTotalGrowthTime))))

(fn StatInitialization
  (params (TMaxMass :type Float%20%28double-precision%29) (TGrowthTime :type Float%20%28double-precision%29) (TDetachParentTime :type Float%20%28double-precision%29))
  (Initialization|SetMaxMass TMaxMass)
  (Initialization|SetGrowthTime TGrowthTime)
  (Initialization|SetDetachParentTime TDetachParentTime))

(fn SetDetachParentTime
  (params (DetachParentMass :type Float%20%28double-precision%29))
  (Variables|Initialization|SetDetachParentTime (Math|Float|Clamp(Float) DetachParentMass 0.0 DetachParentMass)))

(fn GetDetachParentTime
  (return (Variables|Initialization|GetDetachParentTime)))

(fn SetCurrentTime
  (params (CurrentMass :type Float%20%28double-precision%29))
  (Variables|Default|SetCurrentTime CurrentMass))

(fn GetCurrentTime
  (return (Variables|Default|GetCurrentTime)))